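; BP_MainMenu is an actor that shows the main menu and plays the intro widget that follows it.
; BeginPlay creates both widgets, displays the menu with UI-only input and a visible cursor, and binds StartIntro to its click.
; StartIntro adds the intro if the menu's IsOn flag is false.
; A timer then removes the intro, hides the cursor and restores game-only input.
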(event `self.ReceiveBeginPlay`
  (bind _returnvalue (`|CreateWidget` "/Game/Code/WBP_Intro.WBP_Intro_C"))
  (set `self.WBPIntro` _returnvalue)
  (bind _returnvalue_2 (`|CreateWidget` "/Game/Code/WBP_MainMenu.WBP_MainMenu_C"))
  (bind _output_get (set `self.MainMenuWidget` _returnvalue_2))
  (`UserWidget.AddToPlayerScreen` _output_get 0)
  (`UserWidget.AddToViewport` _output_get 0)
  (`WidgetBlueprintLibrary.SetInputMode_UIOnlyEx` (`GameplayStatics.GetPlayerController` 0) null)
  (set `PlayerController.bShowMouseCursor` true (`GameplayStatics.GetPlayerController` 0))
  (add `/Game/Code/WBP_MainMenu.Clicked` (`self.MainMenuWidget`) (delegate `StartIntro`)))

(event `StartIntro`
  (if (not (`/Game/Code/WBP_MainMenu.IsOn` (`self.MainMenuWidget`)))
    (`UserWidget.AddToViewport` (`self.WBPIntro`) 0)
    (`KismetSystemLibrary.K2_SetTimerDelegate` (delegate `RemoveFromView`) 10.0)))

(event `RemoveFromView`
  (`Widget.RemoveFromParent` (`self.WBPIntro`))
  (`WidgetBlueprintLibrary.SetInputMode_GameOnly` (`GameplayStatics.GetPlayerController` 0))
  (set `PlayerController.bShowMouseCursor` false (`GameplayStatics.GetPlayerController` 0)))

(fn `UserConstructionScript`)