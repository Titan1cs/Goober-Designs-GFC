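; Delivery system component that tracks how many items are being carried and the score earned from deliveries.
; Shortly after BeginPlay it takes the HUD reference from the BP_MainMenu actor and refreshes it.
; PickUp raises the carried count without a cap, while Deliver lowers it within a clamped range and always adds score.
; Each event pushes its changed values straight to the HUD, with the max-capacity flag always false.
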(event `self.ReceiveBeginPlay`
  (`KismetSystemLibrary.Delay` 0.01)
  (bind _returnvalue (`GameplayStatics.GetActorOfClass` "/Game/Code/BP_MainMenu.BP_MainMenu_C"))
  (set `self.HUD` (`/Game/Code/BP_MainMenu.Hud` _returnvalue))
  (`self.UpdateHUD` null))

(event `PickUp`
  (bind _output_get (set `self.Carrying` (+ (`self.Carrying`) 1)))
  (`/Game/Code/WBP_HUD.UpdateCarrying` (`self.HUD`) _output_get false))

(event `Deliver`
  (bind _output_get (set `self.Carrying` (`KismetMathLibrary.Clamp` (- (`self.Carrying`) 1) 0 20)))
  (`/Game/Code/WBP_HUD.UpdateCarrying` (`self.HUD`) _output_get false)
  (bind _output_get_2 (set `self.Score` (+ (`self.Score`) 10)))
  (`/Game/Code/WBP_HUD.UpdateScore` (`self.HUD`) _output_get_2))

(event `UpdateHUD`
  (params (OwningPlayer :type "PlayerController Object Reference"))
  (bind _hud (`self.HUD`))
  (`/Game/Code/WBP_HUD.UpdateCarrying` _hud (`self.Carrying`) false)
  (`/Game/Code/WBP_HUD.UpdateScore` _hud (`self.Score`)))